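; Experimental decal actor that lets player input drive an animated sprite through its decal material.
; The construction script creates a dynamic material instance on the decal, and BeginPlay enables input from player 0.
; The MoveRight axis sets TimeScale to stop or play the animation and CharacterFacing to set direction.
; Paired DoOnce nodes reset each other, so parameters update only when input starts or stops.
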(event `self.ReceiveBeginPlay`
  (`self.EnableInput` (`GameplayStatics.GetPlayerController` 0)))

(event `InputAxis|MoveRight`
  (params (AxisValue :type "Float (single-precision)"))
  ;[0 0.9484 1] Movement system for driving sprites
  (if (== AxisValue 0.0)
    (`/Engine/EditorBlueprintResources/StandardMacros.DoOnce` false :!label _label
      (:`Completed`
        (`MaterialInstanceDynamic.SetScalarParameterValue` (`self.DecalMaterialMID`) "TimeScale" 0.0)
        (goto _label_2 :!via `Reset`)))
    (else
      (`/Engine/EditorBlueprintResources/StandardMacros.DoOnce` false :!label _label_2
        (:`Completed`
          (`MaterialInstanceDynamic.SetScalarParameterValue` (`self.DecalMaterialMID`) "CharacterFacing" AxisValue)
          (`MaterialInstanceDynamic.SetScalarParameterValue` (`self.DecalMaterialMID`) "TimeScale" 2.0)
          (goto _label :!via `Reset`))))))

(fn `UserConstructionScript`
  (bind _decal (`self.Decal`))
  (bind _returnvalue (`KismetMaterialLibrary.CreateDynamicMaterialInstance` _decal (`DecalComponent.GetDecalMaterial` _decal)))
  (bind _output_get (set `self.DecalMaterialMID` _returnvalue))
  (`DecalComponent.SetDecalMaterial` (`self.Decal`) _output_get))